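; NPC Blueprint that opens a text dialogue on screen when its Interact event fires.
; Interact creates an NPC_Text widget, copies in this NPC's text lines, text speed and choice arrays, adds it to the viewport and starts the text.
; It then stores the widget in the player's BP_ThirdPersonCharacter as TextChat, giving the character a reference to the active conversation.
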(event `self.ReceiveBeginPlay`)

(event `/Game/Persona6/Blueprints/Interfacer.Interact`
  (bind _returnvalue (`|CreateWidget` "/Game/Persona6/Blueprints/NPC_Text.NPC_Text_C"))
  (set `/Game/Persona6/Blueprints/NPC_Text.Text Array` (`self.Text Array`) _returnvalue)
  (set `/Game/Persona6/Blueprints/NPC_Text.Text Speed` (`self.Text Speed`) _returnvalue)
  (set `/Game/Persona6/Blueprints/NPC_Text.Choice Text Array` (`self.Choice Array`) _returnvalue)
  (set `/Game/Persona6/Blueprints/NPC_Text.Choice Array Array` (`self.Choice Array Array`) _returnvalue)
  (`UserWidget.AddToViewport` _returnvalue 0)
  (`/Game/Persona6/Blueprints/NPC_Text.Start Text` _returnvalue)
  (set `/Game/Persona6/Blueprints/BP_ThirdPersonCharacter.Text Chat` _returnvalue (cast `/Game/Persona6/Blueprints/BP_ThirdPersonCharacter` (`GameplayStatics.GetPlayerCharacter` 0) :!pure true)))

(fn `UserConstructionScript`)
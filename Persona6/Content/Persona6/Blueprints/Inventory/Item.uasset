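; World pickup actor that puts itself into the player's inventory on Interact.
; On spawn or BeginPlay it loads its data table row to set mesh, quantity and physics.
; Interact writes directly into InventorySystem slots, filling a matching partial stack and spilling overflow into the first empty slot.
; It refreshes the character and destroys itself, even when no empty slot exists.
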(event `On Spawn`
  (bind _itemdatacomponent (`self.ItemDataComponent`))
  (bind (_datatable _rowname) (break `DataTableRowHandle` (`/Game/Persona6/Blueprints/Inventory/ItemDataComponent.ItemID` _itemdatacomponent)))
  (`/Engine/EditorBlueprintResources/StandardMacros.IsValid` _datatable :!label _label
    (:`Is Valid`
      (bind _returnvalue (`|GetDataTableRow` _datatable _rowname)
        (:`then`
          (bind _output_get (set `self.Item Structure` _returnvalue))
          (set `self.Quantity` (`/Game/Persona6/Blueprints/Inventory/ItemDataComponent.Quantity` _itemdatacomponent))
          (`StaticMeshComponent.SetStaticMesh` (`self.Item`) (`.ItemMesh_40_FF81DB224B4B672B8BBE27922313BEB4` (break `/Game/Persona6/Blueprints/Inventory/FItemStruct` _output_get)))
          (`PrimitiveComponent.SetSimulatePhysics` (`self.Item`) true))))))

(event `self.ReceiveBeginPlay`
  (goto _label))

(event `/Game/Persona6/Blueprints/Interfacer.Interact`
  (bind (_name _description _thumbnail _itemclass _stacksize) (break `/Game/Persona6/Blueprints/Inventory/FItemStruct` (`self.Item Structure`)))
  (bind _returnvalue (`self.GetComponentByClass` (`GameplayStatics.GetPlayerCharacter` 0) "/Game/Persona6/Blueprints/Inventory/InventorySystem.InventorySystem_C"))
  (for (_array_element _array_index) (`/Game/Persona6/Blueprints/Inventory/InventorySystem.Slot Structure` _returnvalue)
    (bind (_itemid _quantity) (break `/Game/Persona6/Blueprints/Inventory/FSlotStruct` _array_element))
    (if (and (== _itemid _name) (< _quantity _stacksize))
      (set `/Game/Persona6/Blueprints/Inventory/InventorySystem.ItemID` _name _returnvalue)
      (set `self.Array Index` _array_index)
      (`self.Add To Stack`)
      (set `self.Found Slot` true)
      (break)))
  (if (not (`self.Found Slot`))
    (set `/Game/Persona6/Blueprints/Inventory/InventorySystem.ItemID` _name _returnvalue)
    (set `/Game/Persona6/Blueprints/Inventory/InventorySystem.Quantity` (`/Game/Persona6/Blueprints/Inventory/ItemDataComponent.Quantity` (`self.ItemDataComponent`)) _returnvalue)
    (`self.Create New Slot`))
  (`self.K2_DestroyActor`))

(event `Add To Stack`
  (bind _array_index (`self.Array Index`))
  (bind (_name _description _thumbnail _itemclass _stacksize) (break `/Game/Persona6/Blueprints/Inventory/FItemStruct` (`self.Item Structure`)))
  (bind _returnvalue (`self.GetComponentByClass` (`GameplayStatics.GetPlayerCharacter` 0) "/Game/Persona6/Blueprints/Inventory/InventorySystem.InventorySystem_C"))
  (bind _itemid (`/Game/Persona6/Blueprints/Inventory/InventorySystem.ItemID` _returnvalue))
  (bind _slot_structure (`/Game/Persona6/Blueprints/Inventory/InventorySystem.Slot Structure` _returnvalue))
  (bind _output_get (set `/Game/Persona6/Blueprints/Inventory/InventorySystem.Quantity` (+ (`self.Quantity`) (`.Quantity_5_6776D7BB4F7838EB659759A3FAEDA2CE` (break `/Game/Persona6/Blueprints/Inventory/FSlotStruct` (`|GetArrayItem` _slot_structure _array_index)))) _returnvalue))
  (if (> _output_get _stacksize)
    (`KismetArrayLibrary.Array_Set` _slot_structure _array_index (make `/Game/Persona6/Blueprints/Inventory/FSlotStruct` _itemid _stacksize))
    (set `/Game/Persona6/Blueprints/Inventory/InventorySystem.Quantity` (- _output_get _stacksize) _returnvalue)
    (`self.Create New Slot`)
    (else
      (`KismetArrayLibrary.Array_Set` _slot_structure _array_index (make `/Game/Persona6/Blueprints/Inventory/FSlotStruct` _itemid _output_get))))
  (`/Game/Persona6/Blueprints/BP_ThirdPersonCharacter.Refresh` (cast `/Game/Persona6/Blueprints/BP_ThirdPersonCharacter` (`GameplayStatics.GetPlayerCharacter` 0) :!pure true) :!label _label_2))

(event `Create New Slot`
  (bind _returnvalue (`self.GetComponentByClass` (`GameplayStatics.GetPlayerCharacter` 0) "/Game/Persona6/Blueprints/Inventory/InventorySystem.InventorySystem_C"))
  (bind _slot_structure (`/Game/Persona6/Blueprints/Inventory/InventorySystem.Slot Structure` _returnvalue))
  (for (_array_element _array_index) _slot_structure
    (if (== (`.Quantity_5_6776D7BB4F7838EB659759A3FAEDA2CE` (break `/Game/Persona6/Blueprints/Inventory/FSlotStruct` _array_element)) 0)
      (`KismetArrayLibrary.Array_Set` _slot_structure _array_index (make `/Game/Persona6/Blueprints/Inventory/FSlotStruct` (`/Game/Persona6/Blueprints/Inventory/InventorySystem.ItemID` _returnvalue) (`/Game/Persona6/Blueprints/Inventory/InventorySystem.Quantity` _returnvalue)))
      (break)))
  (goto _label_2))

(fn `UserConstructionScript`)
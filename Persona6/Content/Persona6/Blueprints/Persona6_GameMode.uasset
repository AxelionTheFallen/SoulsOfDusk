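; Game mode running one-on-one rock-paper-scissors combat (Strike/Stab/Slash) between the player and an enemy.
; It positions both fighters, builds the heart widget and runs timed rounds, resolving each through CheckResult, CheckCounter and DamageFunction.
; Weapon-type flags scale critical damage, while enemy attacks open offensive, balanced or defensive parry chains that end in a counterattack or failure.
; FinishCombat updates the tagged NPC's quest count and restores exploration state.
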(event `self.ReceiveBeginPlay`
  (set `self.Player` (cast `/Game/Persona6/Blueprints/BP_ThirdPersonCharacter` (`GameplayStatics.GetPlayerCharacter` 0) :!pure true)))

(event `Pre Round Start`
  (bind _current_enemy (`self.Current Enemy`))
  (bind _player (`self.Player`))
  (bind _player_2 (`self.Player`))
  (bind _returnvalue (`self.K2_GetActorLocation` _current_enemy))
  (bind _returnvalue_2 (`self.K2_GetActorLocation` _player))
  (`self.K2_TeleportTo` :`self` _player :`DestLocation` (430.0 -10560.0 88.0))
  (`self.K2_TeleportTo` :`self` _current_enemy :`DestLocation` (230.0 -9950.0 88.0))
  (`self.K2_SetActorRotation` _player (`KismetMathLibrary.FindLookAtRotation` _returnvalue_2 _returnvalue) false)
  (`self.K2_SetActorRotation` _current_enemy (`KismetMathLibrary.FindLookAtRotation` _returnvalue _returnvalue_2) false)
  (bind _returnvalue_3 (`|CreateWidget` "/Game/Persona6/Blueprints/Round_Widget.Round_Widget_C"))
  (bind _output_get (set `self.Combat Widget` _returnvalue_3))
  (set `self.Player Heart` (`|MakeArray` (`/Game/Persona6/Blueprints/Round_Widget.Heart1` _output_get) (`/Game/Persona6/Blueprints/Round_Widget.Heart2` _output_get) (`/Game/Persona6/Blueprints/Round_Widget.Heart3` _output_get) (`/Game/Persona6/Blueprints/Round_Widget.Heart4` _output_get) (`/Game/Persona6/Blueprints/Round_Widget.Heart5` _output_get) (`/Game/Persona6/Blueprints/Round_Widget.Heart6` _output_get) (`/Game/Persona6/Blueprints/Round_Widget.Heart7` _output_get) (`/Game/Persona6/Blueprints/Round_Widget.Heart8` _output_get) (`/Game/Persona6/Blueprints/Round_Widget.Heart9` _output_get) (`/Game/Persona6/Blueprints/Round_Widget.Heart10` _output_get)))
  (set `self.Enemy Heart` (`|MakeArray` (`/Game/Persona6/Blueprints/Round_Widget.Enemy_Heart1` _output_get) (`/Game/Persona6/Blueprints/Round_Widget.Enemy_Heart2` _output_get) (`/Game/Persona6/Blueprints/Round_Widget.Enemy_Heart3` _output_get) (`/Game/Persona6/Blueprints/Round_Widget.Enemy_Heart4` _output_get) (`/Game/Persona6/Blueprints/Round_Widget.Enemy_Heart5` _output_get) (`/Game/Persona6/Blueprints/Round_Widget.Enemy_Heart6` _output_get) (`/Game/Persona6/Blueprints/Round_Widget.Enemy_Heart7` _output_get) (`/Game/Persona6/Blueprints/Round_Widget.Enemy_Heart8` _output_get) (`/Game/Persona6/Blueprints/Round_Widget.Enemy_Heart9` _output_get) (`/Game/Persona6/Blueprints/Round_Widget.Enemy_Heart10` _output_get)))
  (for (_array_element _array_index) (`self.Player Heart`)
    (if (<= _array_index (`/Game/Persona6/Blueprints/BaseCharacter.Max Heart ` _player_2))
      (`Widget.SetVisibility` _array_element "Visible")))
  (`/Game/Persona6/Blueprints/BaseCharacter.Set Heart` _player_2)
  (for (_array_element_2 _array_index_2) (`self.Enemy Heart`)
    (if (<= _array_index_2 (`/Game/Persona6/Blueprints/BaseCharacter.Max Heart ` (`self.Current Enemy`)))
      (`Widget.SetVisibility` _array_element_2 "Visible")))
  (`UserWidget.AddToViewport` (`self.Combat Widget`) 0)
  (`ActorComponent.Deactivate` (`/Game/Persona6/Blueprints/BP_ThirdPersonCharacter.FollowCamera` _player_2))
  (`ActorComponent.Activate` (`/Game/Persona6/Blueprints/BP_ThirdPersonCharacter.CombatCamera` _player_2) false)
  (`self.Close Bools` _player_2)
  (`KismetSystemLibrary.Delay` 1.0)
  (set `self.Combat Can Start` true))

(event `Round Timer`
  (bind _current_time (`self.Current Time`))
  (if (not (`self.Round Ended `))
    (if (<= _current_time (`self.End Time For Enemy`))
      (set `self.Round Ended For Enemy` true))
    (if (<= _current_time 0.0)
      (set `self.Round Ended ` true)
      (`self.Round Ended`)
      (else
        (`KismetSystemLibrary.Delay` 0.01)
        (set `self.Current Time` (- _current_time 0.01))
        (`self.Round Timer`)))))

(event `Player Turn End`
  (set `self.Round Ended For Enemy` true)
  (set `self.Round Ended ` true)
  (`self.Round Ended`))

(event `AI Turn End`
  (bind _parrytype (`/Game/Persona6/Blueprints/Round_Widget.ParryType` (`self.Combat Widget`)))
  (`TextBlock.SetText` _parrytype "E \nN \nE \nM \nY \n \nA \nT \nT \nA \nC \nK \nE \nD")
  (`Widget.SetVisibility` _parrytype "Visible")
  (set `self.Parry` true)
  (set `self.Round Ended For Enemy` true)
  (`self.AI Check Attack`)
  (`KismetSystemLibrary.RetriggerableDelay` 0.75)
  (set `self.Round Ended ` true)
  (if (not (`/Game/Persona6/Blueprints/BP_ThirdPersonCharacter.Selected` (`self.Player`)))
    (`self.Player Turn End`)))

(event `Round Ended`
  (bind _player (`self.Player`))
  (bind _current_enemy (`self.Current Enemy`))
  (bind _scissors (`/Game/Persona6/Blueprints/BaseCharacter.Scissors` _current_enemy))
  (bind _rock (`/Game/Persona6/Blueprints/BaseCharacter.Rock` _current_enemy))
  (bind _paper (`/Game/Persona6/Blueprints/BaseCharacter.Paper` _current_enemy))
  (`/Engine/EditorBlueprintResources/StandardMacros.IsValid` _current_enemy
    (:`Is Valid`
      (`|ExecutionSequence`
        (:`then_0`
          (`self.AI Check Attack`))
        (:`then_1`
          (`self.Check Result` (`/Game/Persona6/Blueprints/BaseCharacter.Rock` _player) _rock _paper _scissors (`/Game/Persona6/Blueprints/BaseCharacter.Edged` _player) (`/Game/Persona6/Blueprints/BaseCharacter.Double Edged` _player) (`/Game/Persona6/Blueprints/BaseCharacter.Secondary Edged` _player) (`/Game/Persona6/Blueprints/BaseCharacter.Pointed` _current_enemy) (`/Game/Persona6/Blueprints/BaseCharacter.Double Pointed` _current_enemy) (`/Game/Persona6/Blueprints/BaseCharacter.Secondary Pointed` _current_enemy)))
        (:`then_2`
          (`self.Check Result` (`/Game/Persona6/Blueprints/BaseCharacter.Paper` _player) _paper _scissors _rock (`/Game/Persona6/Blueprints/BaseCharacter.Pointed` _player) (`/Game/Persona6/Blueprints/BaseCharacter.Double Pointed` _player) (`/Game/Persona6/Blueprints/BaseCharacter.Secondary Pointed` _player) (`/Game/Persona6/Blueprints/BaseCharacter.Blunt` _current_enemy) (`/Game/Persona6/Blueprints/BaseCharacter.Doubled Blunt` _current_enemy) (`/Game/Persona6/Blueprints/BaseCharacter.Secondary Blunt` _current_enemy)))
        (:`then_3`
          (`self.Check Result` (`/Game/Persona6/Blueprints/BaseCharacter.Scissors` _player) _scissors _rock _paper (`/Game/Persona6/Blueprints/BaseCharacter.Blunt` _player) (`/Game/Persona6/Blueprints/BaseCharacter.Doubled Blunt` _player) (`/Game/Persona6/Blueprints/BaseCharacter.Secondary Blunt` _player) (`/Game/Persona6/Blueprints/BaseCharacter.Edged` _current_enemy) (`/Game/Persona6/Blueprints/BaseCharacter.Double Edged` _current_enemy) (`/Game/Persona6/Blueprints/BaseCharacter.Secondary Edged` _current_enemy)))
        (:`then_4`
          (`self.Damage Function`))))))

(event `AI Check Attack`
  (bind _current_enemy (`self.Current Enemy`))
  (bind _enemy_did (`/Game/Persona6/Blueprints/Round_Widget.Enemy_Did` (`self.Combat Widget`)))
  (if (`/Game/Persona6/Blueprints/BaseCharacter.Rock` _current_enemy)
    (`TextBlock.SetText` _enemy_did "Strike")
    (elif (`/Game/Persona6/Blueprints/BaseCharacter.Paper` _current_enemy)
      (`TextBlock.SetText` _enemy_did "Stab")
      (else
        (`TextBlock.SetText` _enemy_did "Slash"))))
  (`Widget.SetVisibility` _enemy_did "Visible"))

(event `Next Round`
  (`/Engine/EditorBlueprintResources/StandardMacros.DoOnce` false :!label _label
    (:`Completed`
      (`KismetSystemLibrary.RetriggerableDelay` 2.0)
      (set `self.Round Ended For Enemy` false)
      (set `self.Round Ended ` false)
      (set `self.Current Time` (`self.Round Time`))
      (`/Game/Persona6/Blueprints/Enemy.Start Round` (`self.Current Enemy`))
      (`self.Round Timer`)
      (`Widget.SetVisibility` (`/Game/Persona6/Blueprints/Round_Widget.Player_Did` (`self.Combat Widget`)) "Hidden")
      (`Widget.SetVisibility` (`/Game/Persona6/Blueprints/Round_Widget.Enemy_Did` (`self.Combat Widget`)) "Hidden")
      (`Widget.SetVisibility` (`/Game/Persona6/Blueprints/Round_Widget.Result` (`self.Combat Widget`)) "Hidden")
      (`KismetSystemLibrary.RetriggerableDelay` 0.5)
      (set `/Game/Persona6/Blueprints/BP_ThirdPersonCharacter.Selected` false (`self.Player`))
      (goto _label :!via `Reset`))))

(event `Finish Combat`
  (bind _current_enemy (`self.Current Enemy`))
  (bind _player (`self.Player`))
  (bind _tags (`Actor.Tags` _current_enemy))
  (if (`KismetArrayLibrary.Array_IsValidIndex` _tags)
    (bind _outactors (`GameplayStatics.GetAllActorsOfClassWithTag` "/Game/Persona6/Blueprints/NPC/NPCS.NPCS_C" (`|GetArrayItem` _tags)))
    (for _array_element _outactors
      _)
    (bind _active_quest_count (`/Game/Persona6/Blueprints/NPC/NPCS.Active Quest Count` _array_element))
    (`/Engine/EditorBlueprintResources/StandardMacros.IncrementInt` _active_quest_count
      (:`  `
        (bind (_datatable _rowname) (break `DataTableRowHandle` (`/Game/Persona6/Blueprints/NPC/Quest_StructComponent.Taken Quests` (`self.GetComponentByClass` _array_element "/Game/Persona6/Blueprints/NPC/Quest_StructComponent.Quest_StructComponent_C"))))
        (bind _returnvalue (`|GetDataTableRow` _datatable _rowname)
          (:`then`
            (if (>= _active_quest_count (`.Count_9_D9EF54D5478DBA0D7E6F17B98680EC4E` (break `/Game/Persona6/Blueprints/NPC/Quests_Structure` _returnvalue)))
              (`KismetArrayLibrary.Array_Set` (`/Game/Persona6/Blueprints/NPC/NPCS.Quest Done Array` _array_element) (`/Game/Persona6/Blueprints/NPC/NPCS.Quest Index` _array_element) true)))))))
  (`self.K2_DestroyActor` _current_enemy)
  (`Widget.RemoveFromParent` (`self.Combat Widget`))
  (set `self.Combat End` false)
  (`self.K2_TeleportTo` _player (`/Game/Persona6/Blueprints/BP_ThirdPersonCharacter.Pre Combat Location` _player) (`/Game/Persona6/Blueprints/BP_ThirdPersonCharacter.Pre Combat Rotation` _player))
  (`CharacterMovementComponent.SetMovementMode` (`Character.CharacterMovement` _player) "MOVE_Walking" 0)
  (`ActorComponent.Deactivate` (`/Game/Persona6/Blueprints/BP_ThirdPersonCharacter.CombatCamera` _player))
  (`ActorComponent.Activate` (`/Game/Persona6/Blueprints/BP_ThirdPersonCharacter.FollowCamera` _player) false)
  (set `/Game/Persona6/Blueprints/BP_ThirdPersonCharacter.Inv Close` true _player)
  (set `/Game/Persona6/Blueprints/BP_ThirdPersonCharacter.Combat Phase` false _player))

(fn `Damage Function`
  (bind _counter_attack (`self.Counter Attack`))
  (bind _parry (`self.Parry`))
  (bind _returnvalue (or (`self.Balanced Parry`) (`self.Offensive Parry`) (`self.Defensive Parry`)))
  (bind _selected (`/Game/Persona6/Blueprints/BP_ThirdPersonCharacter.Selected` (`self.Player`)))
  (bind _result (`/Game/Persona6/Blueprints/Round_Widget.Result` (`self.Combat Widget`)))
  (bind _parrytype (`/Game/Persona6/Blueprints/Round_Widget.ParryType` (`self.Combat Widget`)))
  (if (or _counter_attack (`self.Parry Failed`))
    (if _counter_attack
      (`GameplayStatics.ApplyDamage` (`self.Current Enemy`) (`self.Parry Damage`))
      (else
        (`GameplayStatics.ApplyDamage` (`self.Player`) (`self.AI Parry Damage`))))
    (set `self.Balanced Parry` false)
    (set `self.Defensive Parry` false)
    (set `self.Counter Attack` false)
    (set `self.Parry Failed` false)
    (set `self.Counter Attack` false)
    (set `self.Parry Index` 0)
    (`TextBlock.SetText` _parrytype "")
    (else
      (`Widget.SetVisibility` _result "Visible")
      (if _selected
        (if (`self.Draw`)
          (`TextBlock.SetText` _result "=")
          (set `self.Draw` false)
          (if _parry
            (set `self.Balanced Parry` true)
            (`TextBlock.SetText` _parrytype "B \nA \nL \nA \nN \nC \nE \nD \n \nP \nA \nR \nR \nY")
            (set `self.Parry` false :!label _label)
            (`self.Next Round` :!label _label_2)
            (else
              (`self.Next Round`)))
          (elif (not (`self.Player Won`))
            (`TextBlock.SetText` _result "<" :!label _label_3)
            (if (and _parry _selected)
              (set `self.Defensive Parry` true)
              (`TextBlock.SetText` _parrytype "D \nE \nF \nE \nN \nS \nI \nV \nE \n \nP \nA \nR \nR \nY")
              (goto _label)
              (elif _returnvalue
                (goto _label_2)
                (else
                  (`GameplayStatics.ApplyDamage` (`self.Player`) (`self.AI +Critic Damage`))
                  (`TextBlock.SetText` _parrytype ""))))
            (else
              (`TextBlock.SetText` _result ">")
              (if _parry
                (set `self.Offensive Parry` true)
                (`TextBlock.SetText` _parrytype "O \nF \nF \nE \nN \nS \nI \nV \nE \n \nP \nA \nR \nR \nY")
                (goto _label)
                (elif _returnvalue
                  (goto _label_2)
                  (else
                    (`GameplayStatics.ApplyDamage` (`self.Current Enemy`) (`self.+Critic Damage`))))))))
        (else
          (goto _label_3))))))

(fn `UserConstructionScript`)
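; Base character for Persona6 that tracks Health and converts it into a heart count for display.
; AnyDamage reduces Health, recalculates Heart in ten-point units with a Half flag that is set but never cleared here, then calls SetHeart.
; Non-lethal hits also call NextRound on Persona6_GameMode, while lethal hits set Heart to -1, call SetHeart and destroy the actor.
; SetHeart is an empty event here.
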(event `self.ReceiveAnyDamage`
  (params (Damage :type "Float (single-precision)") (DamageType :type "DamageType Object Reference") (InstigatedBy :type "Controller Object Reference") (DamageCauser :type "Actor Object Reference"))
  (bind _returnvalue (- (`self.Health`) Damage))
  (if (<= _returnvalue 0.0)
    (set `self.Heart` -1.0)
    (`self.Set Heart`)
    (`self.K2_DestroyActor`)
    (else
      (bind _output_get (set `self.Health` _returnvalue))
      (bind _returnvalue_2 (/ (- _output_get 10.0) 10.0))
      (bind _returnvalue_3 (`KismetMathLibrary.FFloor` _returnvalue_2))
      (bind _returnvalue_4 (+ (`KismetMathLibrary.Conv_IntToDouble` _returnvalue_3) 0.5))
      (`/Engine/EditorBlueprintResources/StandardMacros.CompareFloat` _returnvalue_2 _returnvalue_4
        (:`>`
          (set `self.Heart` (+ _returnvalue_3 1)))
        (:`==`
          (set `self.Heart` (+ _returnvalue_4 1.0) :!label _label)
          (set `self.Half` true))
        (:`<`
          (goto _label)))
      (`self.Set Heart`)
      (`/Game/Persona6/Blueprints/Persona6_GameMode.Next Round` (cast `/Game/Persona6/Blueprints/Persona6_GameMode` (`GameplayStatics.GetGameMode`) :!pure true)))))

(event `Set Heart`)

(fn `UserConstructionScript`)
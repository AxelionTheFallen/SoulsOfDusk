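; NPC Blueprint that opens a dialogue, with player choices and an optional quest link, when interacted with.
; Interact creates an NPC_Text widget, fills it with the NPC's lines, text speed, choice data and the quest row name from QuestStructComponent, then starts the text.
; It stores the widget as TextChat on the player's BP_ThirdPersonCharacter and disables that character's movement, with no re-enable in this graph.
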(event `self.ReceiveBeginPlay`)

(event `/Game/Persona6/Blueprints/Interfacer.Interact`
  (params (Location :type "Vector Structure"))
  (bind _asbp_third_person_character (cast `/Game/Persona6/Blueprints/BP_ThirdPersonCharacter` (`GameplayStatics.GetPlayerCharacter` 0) :!pure true))
  (bind _returnvalue (`|CreateWidget` "/Game/Persona6/Blueprints/NPC/NPC_Text.NPC_Text_C"))
  (set `/Game/Persona6/Blueprints/NPC/NPC_Text.Text Array` (`self.Text Array`) _returnvalue)
  (set `/Game/Persona6/Blueprints/NPC/NPC_Text.Text Speed` (`self.Text Speed`) _returnvalue)
  (set `/Game/Persona6/Blueprints/NPC/NPC_Text.Player Choice Text Up Array` (`self.Player Choices Up Array`) _returnvalue)
  (set `/Game/Persona6/Blueprints/NPC/NPC_Text.Player Choice Text Down Array` (`self.Player Choices Down Array`) _returnvalue)
  (set `/Game/Persona6/Blueprints/NPC/NPC_Text.Player Choice Array` (`self.Player Choices Array Array`) _returnvalue)
  (set `/Game/Persona6/Blueprints/NPC/NPC_Text.Player Choice is Quest` (`self.Player Choice is Quest`) _returnvalue)
  (set `/Game/Persona6/Blueprints/NPC/NPC_Text.Quest_ID` (`.RowName` (break `DataTableRowHandle` (`/Game/Persona6/Blueprints/NPC/Quest_StructComponent.Taken Quests` (`self.Quest_StructComponent`)))) _returnvalue)
  (`UserWidget.AddToViewport` _returnvalue 0)
  (`/Game/Persona6/Blueprints/NPC/NPC_Text.Start Text` _returnvalue)
  (set `/Game/Persona6/Blueprints/BP_ThirdPersonCharacter.Text Chat` _returnvalue _asbp_third_person_character)
  (`CharacterMovementComponent.DisableMovement` (`Character.CharacterMovement` _asbp_third_person_character)))

(fn `UserConstructionScript`)
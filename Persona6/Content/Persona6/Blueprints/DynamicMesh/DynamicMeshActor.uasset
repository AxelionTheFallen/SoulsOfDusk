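; A dynamic mesh actor that forms a box which can be carved away at a given world location.
; The construction script resets the mesh, builds a tessellated box with Geometry Script and enables complex-as-simple collision.
; Interact converts the location to component space, builds a sphere-box on a pooled compute mesh and boolean-subtracts it from the component's mesh, then releases the compute meshes.
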(event `/Game/Persona6/Blueprints/Interfacer.Interact`
  (params (Location :type "Vector Structure"))
  (bind _dynamicmeshcomponent (`self.DynamicMeshComponent`))
  (bind _returnvalue (`self.AllocateComputeMesh`))
  (bind _returnvalue_2 (`GeometryScriptLibrary_MeshPrimitiveFunctions.AppendSphereBox` _returnvalue (struct) (`KismetMathLibrary.MakeTransform` (`KismetMathLibrary.InverseTransformLocation` (`SceneComponent.K2_GetComponentToWorld` _dynamicmeshcomponent) Location)) 100.0 6 6 6 "Center" null))
  (bind _returnvalue_3 (`BaseDynamicMeshComponent.GetDynamicMesh` _dynamicmeshcomponent))
  (`GeometryScriptLibrary_MeshBooleanFunctions.ApplyMeshBoolean` _returnvalue_3 (struct) _returnvalue_2 (struct) "Subtract" (struct) null)
  (`self.ReleaseAllComputeMeshes`))

(fn `UserConstructionScript`
  (bind _returnvalue (`BaseDynamicMeshComponent.GetDynamicMesh` (`self.DynamicMeshComponent`)))
  (bind _output_get (set `self.NewVar` _returnvalue))
  (`DynamicMesh.Reset` _output_get)
  (bind _returnvalue_2 (`GeometryScriptLibrary_MeshPrimitiveFunctions.AppendBox` (`self.NewVar`) (struct) (struct) 150.0 150.0 150.0 0 0 0 "Base" null))
  (`GeometryScriptLibrary_MeshSubdivideFunctions.ApplyPNTessellation` _returnvalue_2 (struct) 2 null)
  (`DynamicMeshComponent.SetComplexAsSimpleCollisionEnabled` (`self.DynamicMeshComponent`) true true))
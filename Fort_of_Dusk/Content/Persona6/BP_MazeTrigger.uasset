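; BP_MazeTrigger is a box trigger that starts the maze sequence when BP_ThirdPersonCharacter overlaps it.
; On overlap it calls MazeCameraSet on the character and Timer on the level's BP_MazeGate, then fires LightRepeater.
; LightRepeater runs a timeline once, behind a DoOnce, blending the height fog's opacity, density and falloff from stored values to fixed targets while fading the directional light to zero.
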(event `self.Box.OnComponentBeginOverlap`
  (params (OverlappedComponent :type "PrimitiveComponent Object Reference") (OtherActor :type "Actor Object Reference") (OtherComp :type "PrimitiveComponent Object Reference") (OtherBodyIndex :type Integer) (bFromSweep :type Boolean) (SweepResult :type "HitResult Structure (by ref)"))
  (bind _asbp_third_person_character (cast `/Game/Persona6/Blueprints/BP_ThirdPersonCharacter` OtherActor))
  (`/Game/Persona6/Blueprints/BP_ThirdPersonCharacter.MazeCameraSet` _asbp_third_person_character)
  (bind _returnvalue (`GameplayStatics.GetActorOfClass` "/Game/Persona6/BP_MazeGate.BP_MazeGate_C"))
  (`/Game/Persona6/BP_MazeGate.Timer` _returnvalue)
  (`self.Light Repeater`))

(event `Light Repeater`
  (`/Engine/EditorBlueprintResources/StandardMacros.DoOnce` false
    (:`Completed`
      (bind (_direction _newtrack_0) (`Timeline|Timeline` :!via `PlayFromStart`)
        (:`Update`
          (bind _returnvalue (`GameplayStatics.GetActorOfClass` "/Script/Engine.ExponentialHeightFog"))
          (bind _component (`ExponentialHeightFog.Component` _returnvalue))
          (`ExponentialHeightFogComponent.SetFogMaxOpacity` _component (`KismetMathLibrary.Lerp` (`self.Opacity Value`) 1.0 _newtrack_0))
          (`ExponentialHeightFogComponent.SetFogDensity` _component (`KismetMathLibrary.Lerp` (`self.Fog Density`) 5.0 _newtrack_0))
          (`ExponentialHeightFogComponent.SetFogHeightFalloff` _component (`KismetMathLibrary.Lerp` (`self.Height Falloff`) 1.0 _newtrack_0))
          (bind _returnvalue_2 (`GameplayStatics.GetActorOfClass` "/Script/Engine.DirectionalLight"))
          (`LightComponent.SetIntensity` (`Light.LightComponent` _returnvalue_2) (`KismetMathLibrary.Lerp` (`self.Set Intensity`) 0.0 _newtrack_0)))))))

(fn `UserConstructionScript`)
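; NPC Blueprint for talkable characters and quest givers that open a dialogue widget when the player interacts.
; Interact disables player movement, then a timeline turns the NPC to face the player.
; It then picks default, quest-taken or quest-done lines and passes them, with choice, answer and quest data, to a new NPC_Text widget.
; TalkFinished turns the NPC back to its starting rotation with a second timeline.
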(event `self.ReceiveBeginPlay`
  (set `self.Start Rotation` (`self.K2_GetActorRotation`)))

(event `/Game/Persona6/Blueprints/Interfacer.Interact`
  (params (Location :type "Vector Structure"))
  (bind _quest_index (`self.Quest Index`))
  (`CharacterMovementComponent.DisableMovement` (`Character.CharacterMovement` (cast `/Game/Persona6/Blueprints/BP_ThirdPersonCharacter` (`GameplayStatics.GetPlayerCharacter` 0) :!pure true)))
  (bind (_direction _newtrack_0) (`Timeline|Change to Player Rotation` :!via `PlayFromStart`)
    (:`Update`
      (`self.K2_SetActorRotation` (`KismetMathLibrary.RLerp` (`self.Start Rotation`) (`KismetMathLibrary.FindLookAtRotation` (`self.K2_GetActorLocation`) (`self.K2_GetActorLocation` (`GameplayStatics.GetPlayerCharacter` 0))) _newtrack_0 true)))
    (:`Finished`
      (set `self.Changed Rotation` (`self.K2_GetActorRotation`))
      (if (`self.is Quest Giver`)
        (if (`|GetArrayItem` (`self.Quest Taken Array`) _quest_index)
          (if (`|GetArrayItem` (`self.Quest Done Array`) _quest_index)
            (set `self.Main Text Array` (`self.Quest Done Text Array`))
            (else
              (set `self.Main Text Array` (`self.Quest Taken Text Array`))))
          (else
            (set `self.Main Text Array` (`self.Text Array`) :!label _label)))
        (else
          (goto _label)))
      (bind _returnvalue (`|CreateWidget` "/Game/Persona6/Blueprints/NPC/NPC_Text.NPC_Text_C" null self))
      (set `/Game/Persona6/Blueprints/NPC/NPC_Text.Text Array` (`self.Main Text Array`) _returnvalue)
      (set `/Game/Persona6/Blueprints/NPC/NPC_Text.Text Speed` (`self.Text Speed`) _returnvalue)
      (set `/Game/Persona6/Blueprints/NPC/NPC_Text.Player Choice Text Up Array` (`self.Player Choices Up Array`) _returnvalue)
      (set `/Game/Persona6/Blueprints/NPC/NPC_Text.Player Choice Text Down Array` (`self.Player Choices Down Array`) _returnvalue)
      (set `/Game/Persona6/Blueprints/NPC/NPC_Text.Player Choice Array` (`self.Player Choices Array Array`) _returnvalue)
      (set `/Game/Persona6/Blueprints/NPC/NPC_Text.Player Choice is Quest` (`self.Player Choice is Quest`) _returnvalue)
      (set `/Game/Persona6/Blueprints/NPC/NPC_Text.Quest ID` (`.RowName` (break `DataTableRowHandle` (`/Game/Persona6/Blueprints/NPC/Quest_StructComponent.Taken Quests` (`self.Quest_StructComponent`)))) _returnvalue)
      (set `/Game/Persona6/Blueprints/NPC/NPC_Text.Answer Up Array` (`self.Answer Up Array`) _returnvalue)
      (set `/Game/Persona6/Blueprints/NPC/NPC_Text.Answer Down Array` (`self.Answer Down Array`) _returnvalue)
      (set `/Game/Persona6/Blueprints/NPC/NPC_Text.Player Choice is End` (`self.Player Choice is End`) _returnvalue)
      (set `/Game/Persona6/Blueprints/NPC/NPC_Text.Answer Index Array` (`self.Answer Index Array`) _returnvalue)
      (set `/Game/Persona6/Blueprints/NPC/NPC_Text.is Quest Giver` (`self.is Quest Giver`) _returnvalue)
      (`UserWidget.AddToViewport` _returnvalue 0)
      (`/Game/Persona6/Blueprints/NPC/NPC_Text.Start Text` _returnvalue)
      (set `/Game/Persona6/Blueprints/BP_ThirdPersonCharacter.Text Chat` _returnvalue (cast `/Game/Persona6/Blueprints/BP_ThirdPersonCharacter` (`GameplayStatics.GetPlayerCharacter` 0) :!pure true)))))

(event `Talk Finished`
  (bind (_direction _newtrack_0) (`Timeline|Change to Start Rotation` :!via `PlayFromStart`)
    (:`Update`
      (`self.K2_SetActorRotation` (`KismetMathLibrary.RLerp` (`self.Changed Rotation`) (`self.Start Rotation`) _newtrack_0 true)))))

(fn `UserConstructionScript`)
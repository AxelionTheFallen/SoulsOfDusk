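; Enemy for a rock-paper-scissors style combat game, handling its attack selection and heart display.
; StartRound randomly picks strike, stab or slash every half second, showing the matching combat widget arrow, until the round ends or Sleep is set.
; Each pick has a small random chance to call AITurnEnd on the GameMode, blocked by parry flags.
; SetHeart empties the GameMode's heart bars above current health and draws half hearts.
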(event `Start Round`
  (bind _aspersona_6_game_mode (cast `/Game/Persona6/Blueprints/Persona6_GameMode` (`GameplayStatics.GetGameMode`) :!pure true))
  (bind _combat_widget (`/Game/Persona6/Blueprints/Persona6_GameMode.Combat Widget` _aspersona_6_game_mode))
  (if (and (not (`/Game/Persona6/Blueprints/Persona6_GameMode.Round Ended For Enemy` (cast `/Game/Persona6/Blueprints/Persona6_GameMode` (`GameplayStatics.GetGameMode`) :!pure true))) (not (`self.Sleep`))) :!label _label
    (`self.Close Combat Booleans`)
    (switch `int` (`KismetMathLibrary.RandomIntegerInRange` 0 2)
      (:`0`
        (set `self.Rock` true)
        (`self.VisibilityForArrow` (`/Game/Persona6/Blueprints/Round_Widget.EnemyStrikeArrow` _combat_widget)
          (:`Output`
            _)))
      (:`1`
        (set `self.Paper` true)
        (`self.VisibilityForArrow` (`/Game/Persona6/Blueprints/Round_Widget.EnemyStabArrow` _combat_widget)
          (:`Output`
            _)))
      (:`2`
        (set `self.Scissors` true)
        (`self.VisibilityForArrow` (`/Game/Persona6/Blueprints/Round_Widget.EnemySlashArrow` _combat_widget)
          (:`Output`
            _))))
    (if (and (not (or (`/Game/Persona6/Blueprints/Persona6_GameMode.Defensive Parry` _aspersona_6_game_mode) (`/Game/Persona6/Blueprints/Persona6_GameMode.Balanced Parry` _aspersona_6_game_mode) (`/Game/Persona6/Blueprints/Persona6_GameMode.Offensive Parry` _aspersona_6_game_mode) (`self.Prevent Parry`))) (== (`KismetMathLibrary.RandomIntegerInRange` 0 20) 20))
      (`/Game/Persona6/Blueprints/Persona6_GameMode.AI Turn End` _aspersona_6_game_mode)
      (else
        (`KismetSystemLibrary.Delay` 0.5)
        (goto _label)))))

(event `self.Set Heart`
  (for (_array_element _array_index) (`/Game/Persona6/Blueprints/Persona6_GameMode.Enemy Heart` (cast `/Game/Persona6/Blueprints/Persona6_GameMode` (`GameplayStatics.GetGameMode`) :!pure true))
    (if (and (> _array_index (`self.Heart`)) (<= _array_index (`self.Max Heart `)))
      (`ProgressBar.SetPercent` _array_element 0.0)))
  (if (`self.Half`)
    (`ProgressBar.SetPercent` _array_element 0.5)
    (`ProgressBar.SetPercent` (`|GetArrayItem` (`/Game/Persona6/Blueprints/Persona6_GameMode.Enemy Heart` (cast `/Game/Persona6/Blueprints/Persona6_GameMode` (`GameplayStatics.GetGameMode`) :!pure true)) (`KismetMathLibrary.FTrunc` (`self.Heart`))) 0.5)
    (set `self.Half` false)))

(fn `UserConstructionScript`
  (`parent.UserConstructionScript`))
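; Player inventory system that keeps a 28-slot array of item IDs and quantities, handling pickups and weapon equipping.
; Interacted fills a matching stack or the first empty slot, spills overflow into a new slot, then removes the source actor or widget.
; Equipments reads WeaponsData by stored ItemID, swaps the item into slot 24, and sets the character's weapon mesh and attack-type flag.
; Slot changes call Refresh on the character.
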(event `self.ReceiveBeginPlay`
  (`KismetArrayLibrary.Array_Resize` (`self.Slot Structure`) 28))

(event `Interacted`
  (params (B :type "/Game/Persona6/Blueprints/Inventory/FItemStruct Structure") (Actor :type "Actor Object Reference") (Quantity :type Integer) (`Is Item` :type Boolean) (Widget :type "Widget Object Reference"))
  (bind ((`Name_32_2AEA4BDF4BA7CA203D9C298DB65B2A96` _name) (`StackSize_15_B5462DD949531CB827C57F8D7D96DE2D` _stacksize)) (break `/Game/Persona6/Blueprints/Inventory/FItemStruct` B))
  (for (_array_element _array_index) (`self.Slot Structure`)
    (bind (_itemid _quantity) (break `/Game/Persona6/Blueprints/Inventory/FSlotStruct` _array_element))
    (if (and (== _itemid _name) (< _quantity _stacksize))
      (set `self.ItemID` _name)
      (set `self.Array Index` _array_index)
      (`self.Add To Stack1` Quantity _stacksize)
      (set `self.Found Slot` true)
      (break)))
  (if (not (`self.Found Slot`))
    (set `self.ItemID` _name)
    (set `self.Quantity` Quantity)
    (`self.Create New Slot`))
  (set `self.Found Slot` false)
  (if `Is Item`
    (`Actor.K2_DestroyActor` Actor)
    (else
      (`Widget.RemoveFromParent` Widget))))

(event `Equipments`
  (params (Quantity :type Integer) (`Item Index` :type Integer) (Slot :type "/Game/Persona6/Blueprints/Inventory/FItemStruct Structure"))
  (bind _asbp_third_person_character (cast `/Game/Persona6/Blueprints/Characters/Player/BP_ThirdPersonCharacter` (`GameplayStatics.GetPlayerCharacter` 0) :!pure true))
  (bind _returnvalue (`|GetDataTableRow` "/Game/Persona6/Blueprints/Inventory/WeaponsData.WeaponsData" (`self.ItemID`))
    (:`then`
      (bind (_doubleedged _mainedge _secondaryedge _doublepointed _mainpointed _secondarypointed _doubleblunt _mainblunt _secondaryblunt) (break `/Game/Persona6/Blueprints/Inventory/WeaponStruct` _returnvalue))
      (for (_array_element _array_index) (`|MakeArray` _doubleedged _mainedge _secondaryedge _doublepointed _mainpointed _secondarypointed _doubleblunt _mainblunt _secondaryblunt)
        (if _array_element
          (`self.Change Equipment Slot` Quantity `Item Index` Slot)
          (`StaticMeshComponent.SetStaticMesh` (`/Game/Persona6/Blueprints/Characters/Player/BP_ThirdPersonCharacter.Weapon` _asbp_third_person_character) (`.ItemMesh_40_FF81DB224B4B672B8BBE27922313BEB4` (break `/Game/Persona6/Blueprints/Inventory/FItemStruct` Slot)))
          (set `/Game/Persona6/Blueprints/Characters/BaseCharacter.Double Edged` false _asbp_third_person_character)
          (set `/Game/Persona6/Blueprints/Characters/BaseCharacter.Edged` false _asbp_third_person_character)
          (set `/Game/Persona6/Blueprints/Characters/BaseCharacter.Secondary Edged` false _asbp_third_person_character)
          (set `/Game/Persona6/Blueprints/Characters/BaseCharacter.Double Pointed` false _asbp_third_person_character)
          (set `/Game/Persona6/Blueprints/Characters/BaseCharacter.Pointed` false _asbp_third_person_character)
          (set `/Game/Persona6/Blueprints/Characters/BaseCharacter.Secondary Pointed` false _asbp_third_person_character)
          (set `/Game/Persona6/Blueprints/Characters/BaseCharacter.Doubled Blunt` false _asbp_third_person_character)
          (set `/Game/Persona6/Blueprints/Characters/BaseCharacter.Blunt` false _asbp_third_person_character)
          (set `/Game/Persona6/Blueprints/Characters/BaseCharacter.Secondary Blunt` false _asbp_third_person_character)
          (switch `int` _array_index
            (:`0`
              (set `/Game/Persona6/Blueprints/Characters/BaseCharacter.Double Edged` true _asbp_third_person_character))
            (:`1`
              (set `/Game/Persona6/Blueprints/Characters/BaseCharacter.Edged` true _asbp_third_person_character))
            (:`2`
              (set `/Game/Persona6/Blueprints/Characters/BaseCharacter.Secondary Edged` true _asbp_third_person_character))
            (:`3`
              (set `/Game/Persona6/Blueprints/Characters/BaseCharacter.Double Pointed` true _asbp_third_person_character))
            (:`4`
              (set `/Game/Persona6/Blueprints/Characters/BaseCharacter.Pointed` true _asbp_third_person_character))
            (:`5`
              (set `/Game/Persona6/Blueprints/Characters/BaseCharacter.Secondary Pointed` true _asbp_third_person_character))
            (:`6`
              (set `/Game/Persona6/Blueprints/Characters/BaseCharacter.Doubled Blunt` true _asbp_third_person_character))
            (:`7`
              (set `/Game/Persona6/Blueprints/Characters/BaseCharacter.Blunt` true _asbp_third_person_character))
            (:`8`
              (set `/Game/Persona6/Blueprints/Characters/BaseCharacter.Secondary Blunt` true _asbp_third_person_character))))))))

(event `Change Equipment Slot`
  (params (Quantiy :type Integer) (`Item Index` :type Integer) (Slot :type "/Game/Persona6/Blueprints/Inventory/FItemStruct Structure"))
  (bind ((`Name_32_2AEA4BDF4BA7CA203D9C298DB65B2A96` _name)) (break `/Game/Persona6/Blueprints/Inventory/FItemStruct` Slot))
  (bind _slot_structure (`self.Slot Structure`))
  (bind _output (`|GetArrayItem` _slot_structure 24))
  (if (!= (`.ItemId_7_2D41BED74C8CC8988AD074873717D6BC` (break `/Game/Persona6/Blueprints/Inventory/FSlotStruct` _output)) "None")
    (bind _output_get (set `self.Equipment Inf` _output))
    (`KismetArrayLibrary.Array_Set` _slot_structure 24 (make `/Game/Persona6/Blueprints/Inventory/FSlotStruct` _name))
    (`KismetArrayLibrary.Array_Set` _slot_structure `Item Index` (make `/Game/Persona6/Blueprints/Inventory/FSlotStruct` (break `/Game/Persona6/Blueprints/Inventory/FSlotStruct` _output_get) 1))
    (else
      (`KismetArrayLibrary.Array_Set` _slot_structure 24 (make `/Game/Persona6/Blueprints/Inventory/FSlotStruct` _name))
      (`KismetArrayLibrary.Array_Set` _slot_structure `Item Index` (make `/Game/Persona6/Blueprints/Inventory/FSlotStruct` "None"))))
  (`/Game/Persona6/Blueprints/Characters/Player/BP_ThirdPersonCharacter.Refresh` (cast `/Game/Persona6/Blueprints/Characters/Player/BP_ThirdPersonCharacter` (`GameplayStatics.GetPlayerCharacter` 0) :!pure true)))

(fn `Add To Stack1`
  (params (Quantity :type Integer) (`Stack Sİze` :type Integer))
  (bind _array_index (`self.Array Index`))
  (bind _itemid (`self.ItemID`))
  (bind _slot_structure (`self.Slot Structure`))
  (bind _output_get (set `self.Quantity` (+ Quantity (`.Quantity_5_6776D7BB4F7838EB659759A3FAEDA2CE` (break `/Game/Persona6/Blueprints/Inventory/FSlotStruct` (`|GetArrayItem` _slot_structure _array_index))))))
  (if (> _output_get `Stack Sİze`)
    (`KismetArrayLibrary.Array_Set` _slot_structure _array_index (make `/Game/Persona6/Blueprints/Inventory/FSlotStruct` _itemid `Stack Sİze`))
    (set `self.Quantity` (- _output_get `Stack Sİze`))
    (`self.Create New Slot`)
    (else
      (`KismetArrayLibrary.Array_Set` _slot_structure _array_index (make `/Game/Persona6/Blueprints/Inventory/FSlotStruct` _itemid _output_get))))
  (`/Game/Persona6/Blueprints/Characters/Player/BP_ThirdPersonCharacter.Refresh` (cast `/Game/Persona6/Blueprints/Characters/Player/BP_ThirdPersonCharacter` (`GameplayStatics.GetPlayerCharacter` 0) :!pure true)))

(fn `Create New Slot`
  (bind _slot_structure (`self.Slot Structure`))
  (for (_array_element _array_index) _slot_structure
    (if (== (`.Quantity_5_6776D7BB4F7838EB659759A3FAEDA2CE` (break `/Game/Persona6/Blueprints/Inventory/FSlotStruct` _array_element)) 0)
      (`KismetArrayLibrary.Array_Set` _slot_structure _array_index (make `/Game/Persona6/Blueprints/Inventory/FSlotStruct` (`self.ItemID`) (`self.Quantity`)))
      (break)))
  (`/Game/Persona6/Blueprints/Characters/Player/BP_ThirdPersonCharacter.Refresh` (cast `/Game/Persona6/Blueprints/Characters/Player/BP_ThirdPersonCharacter` (`GameplayStatics.GetPlayerCharacter` 0) :!pure true)))
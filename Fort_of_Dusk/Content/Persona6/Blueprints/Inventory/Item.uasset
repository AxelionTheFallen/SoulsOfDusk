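; Item is a world pickup actor for the inventory system, built from an ItemDataComponent row reference and quantity.
; On BeginPlay or OnSpawn it looks up that data table row, caches the item structure and quantity, then applies the mesh and scale and enables physics.
; Interact passes the structure, quantity and itself to the InventorySystem component on player character 0.
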(event `On Spawn`
  (bind _item (`self.Item`))
  (bind _itemdatacomponent (`self.ItemDataComponent`))
  (bind (_datatable _rowname) (break `DataTableRowHandle` (`/Game/Persona6/Blueprints/Inventory/ItemDataComponent.ItemID` _itemdatacomponent)))
  (`/Engine/EditorBlueprintResources/StandardMacros.IsValid` _datatable :!label _label
    (:`Is Valid`
      (bind _returnvalue (`|GetDataTableRow` _datatable _rowname)
        (:`then`
          (bind _output_get (set `self.Item Structure` _returnvalue))
          (set `self.Quantity` (`/Game/Persona6/Blueprints/Inventory/ItemDataComponent.Quantity` _itemdatacomponent))
          (bind ((`ItemMesh_40_FF81DB224B4B672B8BBE27922313BEB4` _itemmesh) (`ItemScale_68_EE7A1CA342C68F4405EA209D51BBB29B` _itemscale)) (break `/Game/Persona6/Blueprints/Inventory/FItemStruct` _output_get))
          (`StaticMeshComponent.SetStaticMesh` (`self.Item`) _itemmesh)
          (`PrimitiveComponent.SetSimulatePhysics` _item true)
          (`SceneComponent.SetRelativeScale3D` _item _itemscale))))))

(event `self.ReceiveBeginPlay`
  (goto _label))

(event `/Game/Persona6/Blueprints/Interfacer.Interact`
  (params (Location :type "Vector Structure"))
  (`/Game/Persona6/Blueprints/Inventory/InventorySystem.Interacted` (`self.GetComponentByClass` (`GameplayStatics.GetPlayerCharacter` 0) "/Game/Persona6/Blueprints/Inventory/InventorySystem.InventorySystem_C") (`self.Item Structure`) self (`self.Quantity`) true null))

(fn `UserConstructionScript`)
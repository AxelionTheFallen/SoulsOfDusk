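; Game mode that runs timed rock-paper-scissors duels (Strike, Stab, Slash) between the player and an enemy.
; PreRoundStart stages the arena, camera and UI, while a recursive Delay timer counts down each round.
; RoundEnded feeds choices through CheckResult and CheckCounter into DamageFunction, resolving weapon-type criticals, parry chains and magic.
; NextRound ticks magic effects and restarts the timer; FinishCombat updates quest progress and returns the player.
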(event `self.ReceiveBeginPlay`
  (bind _output_get (set `self.Player` (cast `/Game/Persona6/Blueprints/Characters/Player/BP_ThirdPersonCharacter` (`GameplayStatics.GetPlayerCharacter` 0) :!pure true)))
  (set `self.Magic Component` (`self.GetComponentByClass` _output_get "/Game/Persona6/Blueprints/Magics/Magic_Component.Magic_Component_C")))

(event `Pre Round Start`
  (bind _current_enemy (`self.Current Enemy`))
  (bind _current_enemy_2 (`self.Current Enemy`))
  (bind _player (`self.Player`))
  (bind _current_enemy_3 (`self.Current Enemy`))
  (bind _player_2 (`self.Player`))
  (bind _returnvalue (`self.K2_GetActorLocation` _current_enemy_2))
  (bind _returnvalue_2 (`self.K2_GetActorLocation` _player))
  (`MovementComponent.StopMovementImmediately` (`Character.CharacterMovement` _current_enemy))
  (set `/Game/Persona6/Blueprints/Characters/NPC/Agressive/Skeleton.Walking` false (cast `/Game/Persona6/Blueprints/Characters/NPC/Agressive/Skeleton` _current_enemy :!pure true))
  (`self.K2_TeleportTo` :`self` _player :`DestLocation` (430.0 -10560.0 88.0))
  (`self.K2_TeleportTo` :`self` _current_enemy_2 :`DestLocation` (230.0 -9950.0 88.0))
  (`self.K2_SetActorRotation` _player (`KismetMathLibrary.FindLookAtRotation` _returnvalue_2 _returnvalue) false)
  (`self.K2_SetActorRotation` _current_enemy_2 (`KismetMathLibrary.FindLookAtRotation` _returnvalue _returnvalue_2) false)
  (bind _returnvalue_3 (`|CreateWidget` "/Game/Persona6/Blueprints/Round_Widget.Round_Widget_C"))
  (bind _output_get (set `self.Combat Widget` _returnvalue_3))
  (set `self.Player Heart` (`|MakeArray` (`/Game/Persona6/Blueprints/Round_Widget.Heart1` _output_get) (`/Game/Persona6/Blueprints/Round_Widget.Heart2` _output_get) (`/Game/Persona6/Blueprints/Round_Widget.Heart3` _output_get) (`/Game/Persona6/Blueprints/Round_Widget.Heart4` _output_get) (`/Game/Persona6/Blueprints/Round_Widget.Heart5` _output_get) (`/Game/Persona6/Blueprints/Round_Widget.Heart6` _output_get) (`/Game/Persona6/Blueprints/Round_Widget.Heart7` _output_get) (`/Game/Persona6/Blueprints/Round_Widget.Heart8` _output_get) (`/Game/Persona6/Blueprints/Round_Widget.Heart9` _output_get) (`/Game/Persona6/Blueprints/Round_Widget.Heart10` _output_get)))
  (set `self.Enemy Heart` (`|MakeArray` (`/Game/Persona6/Blueprints/Round_Widget.Enemy_Heart1` _output_get) (`/Game/Persona6/Blueprints/Round_Widget.Enemy_Heart2` _output_get) (`/Game/Persona6/Blueprints/Round_Widget.Enemy_Heart3` _output_get) (`/Game/Persona6/Blueprints/Round_Widget.Enemy_Heart4` _output_get) (`/Game/Persona6/Blueprints/Round_Widget.Enemy_Heart5` _output_get) (`/Game/Persona6/Blueprints/Round_Widget.Enemy_Heart6` _output_get) (`/Game/Persona6/Blueprints/Round_Widget.Enemy_Heart7` _output_get) (`/Game/Persona6/Blueprints/Round_Widget.Enemy_Heart8` _output_get) (`/Game/Persona6/Blueprints/Round_Widget.Enemy_Heart9` _output_get) (`/Game/Persona6/Blueprints/Round_Widget.Enemy_Heart10` _output_get)))
  (for (_array_element _array_index) (`self.Player Heart`)
    (if (<= _array_index (`/Game/Persona6/Blueprints/Characters/BaseCharacter.Max Heart ` _player_2))
      (`Widget.SetVisibility` _array_element "Visible")))
  (`/Game/Persona6/Blueprints/Characters/BaseCharacter.Set Heart` _player_2)
  (for (_array_element_2 _array_index_2) (`self.Enemy Heart`)
    (if (<= _array_index_2 (`/Game/Persona6/Blueprints/Characters/BaseCharacter.Max Heart ` _current_enemy_3))
      (`Widget.SetVisibility` _array_element_2 "Visible")))
  (`UserWidget.AddToViewport` (`self.Combat Widget`) 0)
  (`ActorComponent.Deactivate` (`/Game/Persona6/Blueprints/Characters/Player/BP_ThirdPersonCharacter.FollowCamera` _player_2))
  (`ActorComponent.Activate` (`/Game/Persona6/Blueprints/Characters/Player/BP_ThirdPersonCharacter.CombatCamera` _player_2) false)
  (`self.Close Bools` _player_2)
  (`SceneComponent.SetVisibility` (`/Game/Persona6/Blueprints/Characters/BaseCharacter.3D Combat Widget` _current_enemy_3) true false)
  (bind _output_get_2 (set `self.Round Time` (+ (`self.Default Round Time`) (- (`/Game/Persona6/Blueprints/Characters/BaseCharacter.Speed` _player_2) (`/Game/Persona6/Blueprints/Characters/BaseCharacter.Speed` _current_enemy_3)))))
  (set `self.Current Time` _output_get_2)
  (`KismetSystemLibrary.Delay` 1.0)
  (set `self.Combat Can Start` true))

(event `Round Timer`
  (bind _current_time (`self.Current Time`))
  (if (not (`self.Round Ended `))
    (if (<= _current_time (`self.End Time For Enemy`))
      (set `self.Round Ended For Enemy` true))
    (if (<= _current_time 0.0)
      (set `self.Round Ended ` true)
      (`self.Round Ended`)
      (else
        (`KismetSystemLibrary.Delay` 0.01)
        (set `self.Current Time` (- _current_time 0.01))
        (`self.Round Timer`)))))

(event `Player Turn End`
  (set `self.Round Ended For Enemy` true)
  (set `self.Round Ended ` true)
  (`self.Round Ended`))

(event `AI Turn End`
  (bind _parrytype (`/Game/Persona6/Blueprints/Round_Widget.ParryType` (`self.Combat Widget`)))
  (`TextBlock.SetText` _parrytype "E \nN \nE \nM \nY \n \nA \nT \nT \nA \nC \nK \nE \nD")
  (`Widget.SetVisibility` _parrytype "Visible")
  (set `self.Parry` true)
  (set `self.Current Time` (+ (`self.Current Time`) 1.0)))

(event `AI Turn End2`
  (set `self.Round Ended For Enemy` true)
  (`self.AI Check Attack`)
  (set `self.Round Ended ` true)
  (if (not (`/Game/Persona6/Blueprints/Characters/Player/BP_ThirdPersonCharacter.Selected` (`self.Player`)))
    (`self.Player Turn End`)))

(event `Round Ended`
  (bind _player (`self.Player`))
  (bind _current_enemy (`self.Current Enemy`))
  (bind _scissors (`/Game/Persona6/Blueprints/Characters/BaseCharacter.Scissors` _current_enemy))
  (bind _rock (`/Game/Persona6/Blueprints/Characters/BaseCharacter.Rock` _current_enemy))
  (bind _paper (`/Game/Persona6/Blueprints/Characters/BaseCharacter.Paper` _current_enemy))
  (`/Engine/EditorBlueprintResources/StandardMacros.IsValid` _current_enemy
    (:`Is Valid`
      (`|ExecutionSequence`
        (:`then_0`
          (`self.AI Check Attack`))
        (:`then_1`
          (`self.Check Result` (`/Game/Persona6/Blueprints/Characters/BaseCharacter.Rock` _player) _rock _paper _scissors (`/Game/Persona6/Blueprints/Characters/BaseCharacter.Edged` _player) (`/Game/Persona6/Blueprints/Characters/BaseCharacter.Double Edged` _player) (`/Game/Persona6/Blueprints/Characters/BaseCharacter.Secondary Edged` _player) (`/Game/Persona6/Blueprints/Characters/BaseCharacter.Pointed` _current_enemy) (`/Game/Persona6/Blueprints/Characters/BaseCharacter.Double Pointed` _current_enemy) (`/Game/Persona6/Blueprints/Characters/BaseCharacter.Secondary Pointed` _current_enemy)))
        (:`then_2`
          (`self.Check Result` (`/Game/Persona6/Blueprints/Characters/BaseCharacter.Paper` _player) _paper _scissors _rock (`/Game/Persona6/Blueprints/Characters/BaseCharacter.Pointed` _player) (`/Game/Persona6/Blueprints/Characters/BaseCharacter.Double Pointed` _player) (`/Game/Persona6/Blueprints/Characters/BaseCharacter.Secondary Pointed` _player) (`/Game/Persona6/Blueprints/Characters/BaseCharacter.Blunt` _current_enemy) (`/Game/Persona6/Blueprints/Characters/BaseCharacter.Doubled Blunt` _current_enemy) (`/Game/Persona6/Blueprints/Characters/BaseCharacter.Secondary Blunt` _current_enemy)))
        (:`then_3`
          (`self.Check Result` (`/Game/Persona6/Blueprints/Characters/BaseCharacter.Scissors` _player) _scissors _rock _paper (`/Game/Persona6/Blueprints/Characters/BaseCharacter.Blunt` _player) (`/Game/Persona6/Blueprints/Characters/BaseCharacter.Doubled Blunt` _player) (`/Game/Persona6/Blueprints/Characters/BaseCharacter.Secondary Blunt` _player) (`/Game/Persona6/Blueprints/Characters/BaseCharacter.Edged` _current_enemy) (`/Game/Persona6/Blueprints/Characters/BaseCharacter.Double Edged` _current_enemy) (`/Game/Persona6/Blueprints/Characters/BaseCharacter.Secondary Edged` _current_enemy)))
        (:`then_4`
          (`self.Damage Function`))))))

(event `AI Check Attack`
  (bind _current_enemy (`self.Current Enemy`))
  (bind _current_enemy_2 (`self.Current Enemy`))
  (bind _enemy_did (`/Game/Persona6/Blueprints/Round_Widget.Enemy_Did` (`self.Combat Widget`)))
  (bind _asenemy_attack_choose_widget (cast `/Game/Persona6/Blueprints/Characters/NPC/Agressive/EnemyAttackChooseWidget` (`WidgetComponent.GetWidget` (`/Game/Persona6/Blueprints/Characters/BaseCharacter.3D Combat Widget` _current_enemy)) :!pure true))
  (`Widget.SetVisibility` _enemy_did "Visible")
  (if (`/Game/Persona6/Blueprints/Characters/BaseCharacter.Rock` _current_enemy_2)
    (`TextBlock.SetText` _enemy_did "Strike")
    (`Character.PlayAnimMontage` _current_enemy "/Game/Persona6/Animations/AnimationSquences/Skeleton_Attack_Strike_Montage.Skeleton_Attack_Strike_Montage" 1.0 "None")
    (set `self.Enemy WidgetAnim` (`/Game/Persona6/Blueprints/Characters/NPC/Agressive/EnemyAttackChooseWidget.Strike` _asenemy_attack_choose_widget))
    (elif (`/Game/Persona6/Blueprints/Characters/BaseCharacter.Paper` _current_enemy_2)
      (`TextBlock.SetText` _enemy_did "Stab")
      (`Character.PlayAnimMontage` _current_enemy "/Game/Persona6/Animations/AnimationSquences/Skeleton_Attack_Stab_Montage.Skeleton_Attack_Stab_Montage" 1.0 "None")
      (set `self.Enemy WidgetAnim` (`/Game/Persona6/Blueprints/Characters/NPC/Agressive/EnemyAttackChooseWidget.Stab` _asenemy_attack_choose_widget))
      (else
        (`TextBlock.SetText` _enemy_did "Slash")
        (`Character.PlayAnimMontage` _current_enemy "/Game/Persona6/Animations/AnimationSquences/Skeleton_Attack_Slash_Montage.Skeleton_Attack_Slash_Montage" 1.0 "None")
        (set `self.Enemy WidgetAnim` (`/Game/Persona6/Blueprints/Characters/NPC/Agressive/EnemyAttackChooseWidget.Slash` _asenemy_attack_choose_widget)))))
  (`UserWidget.PlayAnimation` _asenemy_attack_choose_widget (`self.Enemy WidgetAnim`) 0.0 1 "Forward" 1.0 false)
  (`KismetSystemLibrary.Delay` 0.2)
  (`UserWidget.PlayAnimationReverse` _asenemy_attack_choose_widget (`self.Enemy WidgetAnim`) 0.2 false))

(event `Next Round`
  (bind _round_time (`self.Round Time`))
  (bind _magic_component (`self.Magic Component`))
  (bind _magic_active (`/Game/Persona6/Blueprints/Magics/Magic_Component.Magic Active` _magic_component))
  (bind _magic_turn (`/Game/Persona6/Blueprints/Magics/Magic_Component.Magic Turn` _magic_component))
  (`/Engine/EditorBlueprintResources/StandardMacros.DoOnce` false :!label _label
    (:`Completed`
      (`KismetSystemLibrary.RetriggerableDelay` 0.4)
      (for (_array_element _array_index) _magic_active
        (if _array_element
          (bind _returnvalue (- (`|GetArrayItem` _magic_turn _array_index) 1))
          (if (<= _returnvalue 0)
            (`KismetArrayLibrary.Array_Set` _magic_turn _array_index)
            (`KismetArrayLibrary.Array_Set` _magic_active _array_index)
            (else
              (`KismetArrayLibrary.Array_Set` _magic_turn _array_index _returnvalue)
              (`GameplayStatics.ApplyDamage` (`self.Current Enemy`) (`|GetArrayItem` (`/Game/Persona6/Blueprints/Magics/Magic_Component.Affliction Damage` _magic_component) _array_index))))))
      (`KismetSystemLibrary.RetriggerableDelay` 0.4)
      (set `self.Round Ended For Enemy` false)
      (set `self.Round Ended ` false)
      (if (`|GetArrayItem` (`/Game/Persona6/Blueprints/Magics/Magic_Component.Magic Active` (`self.Magic Component`)) 3)
        (set `self.Round Time` (+ _round_time 2.0))
        (else
          (set `self.Round Time` (`self.Default Round Time`))))
      (set `self.Current Time` _round_time)
      (`/Game/Persona6/Blueprints/Characters/NPC/Agressive/Enemy.Start Round` (`self.Current Enemy`))
      (`self.Round Timer`)
      (`Widget.SetVisibility` (`/Game/Persona6/Blueprints/Round_Widget.Player_Did` (`self.Combat Widget`)) "Hidden")
      (`Widget.SetVisibility` (`/Game/Persona6/Blueprints/Round_Widget.Enemy_Did` (`self.Combat Widget`)) "Hidden")
      (`Widget.SetVisibility` (`/Game/Persona6/Blueprints/Round_Widget.Result` (`self.Combat Widget`)) "Hidden")
      (`Widget.SetVisibility` (`/Game/Persona6/Blueprints/Characters/Player/PlayerAttackChooseWidget.Arow3` (cast `/Game/Persona6/Blueprints/Characters/Player/PlayerAttackChooseWidget` (`WidgetComponent.GetWidget` (`/Game/Persona6/Blueprints/Characters/BaseCharacter.3D Combat Widget` (`self.Player`))) :!pure true)) "Hidden")
      (`Widget.SetVisibility` (`/Game/Persona6/Blueprints/Characters/Player/PlayerAttackChooseWidget.Arow1` (cast `/Game/Persona6/Blueprints/Characters/Player/PlayerAttackChooseWidget` (`WidgetComponent.GetWidget` (`/Game/Persona6/Blueprints/Characters/BaseCharacter.3D Combat Widget` (`self.Player`))) :!pure true)) "Hidden")
      (`Widget.SetVisibility` (`/Game/Persona6/Blueprints/Characters/Player/PlayerAttackChooseWidget.Arow2` (cast `/Game/Persona6/Blueprints/Characters/Player/PlayerAttackChooseWidget` (`WidgetComponent.GetWidget` (`/Game/Persona6/Blueprints/Characters/BaseCharacter.3D Combat Widget` (`self.Player`))) :!pure true)) "Hidden")
      (`KismetSystemLibrary.RetriggerableDelay` 0.5)
      (set `/Game/Persona6/Blueprints/Characters/Player/BP_ThirdPersonCharacter.Selected` false (`self.Player`))
      (goto _label :!via `Reset`))))

(event `Finish Combat`
  (bind _current_enemy (`self.Current Enemy`))
  (bind _player (`self.Player`))
  (bind _tags (`Actor.Tags` _current_enemy))
  (if (`KismetArrayLibrary.Array_IsValidIndex` _tags)
    (bind _outactors (`GameplayStatics.GetAllActorsOfClassWithTag` "/Game/Persona6/Blueprints/Characters/NPC/Mob/NPCS.NPCS_C" (`|GetArrayItem` _tags)))
    (for _array_element _outactors
      _)
    (bind _active_quest_count (`/Game/Persona6/Blueprints/Characters/NPC/Mob/NPCS.Active Quest Count` _array_element))
    (`/Engine/EditorBlueprintResources/StandardMacros.IncrementInt` _active_quest_count
      (:`  `
        (bind (_datatable _rowname) (break `DataTableRowHandle` (`/Game/Persona6/Blueprints/Characters/NPC/Mob/Quest_StructComponent.Taken Quests` (`self.GetComponentByClass` _array_element "/Game/Persona6/Blueprints/Characters/NPC/Mob/Quest_StructComponent.Quest_StructComponent_C"))))
        (bind _returnvalue (`|GetDataTableRow` _datatable _rowname)
          (:`then`
            (if (>= _active_quest_count (`.Count_9_D9EF54D5478DBA0D7E6F17B98680EC4E` (break `/Game/Persona6/Blueprints/Characters/NPC/Mob/Quests_Structure` _returnvalue)))
              (`KismetArrayLibrary.Array_Set` (`/Game/Persona6/Blueprints/Characters/NPC/Mob/NPCS.Quest Done Array` _array_element) (`/Game/Persona6/Blueprints/Characters/NPC/Mob/NPCS.Quest Index` _array_element) true)))))))
  (`self.K2_DestroyActor` _current_enemy)
  (`Widget.RemoveFromParent` (`self.Combat Widget`))
  (set `self.Combat End` false)
  (`self.K2_TeleportTo` _player (`/Game/Persona6/Blueprints/Characters/Player/BP_ThirdPersonCharacter.Pre Combat Location` _player) (`/Game/Persona6/Blueprints/Characters/Player/BP_ThirdPersonCharacter.Pre Combat Rotation` _player))
  (`ActorComponent.Deactivate` (`/Game/Persona6/Blueprints/Characters/Player/BP_ThirdPersonCharacter.CombatCamera` _player))
  (`ActorComponent.Activate` (`/Game/Persona6/Blueprints/Characters/Player/BP_ThirdPersonCharacter.FollowCamera` _player) false)
  (set `/Game/Persona6/Blueprints/Characters/Player/BP_ThirdPersonCharacter.Inv Close` true _player)
  (set `/Game/Persona6/Blueprints/Characters/Player/BP_ThirdPersonCharacter.Combat Phase` false _player)
  (`SceneComponent.SetVisibility` (`/Game/Persona6/Blueprints/Characters/BaseCharacter.3D Combat Widget` (`self.Player`)) false false))

(fn `Damage Function`
  (bind _counter_attack (`self.Counter Attack`))
  (bind _player (`self.Player`))
  (bind _player_2 (`self.Player`))
  (bind _current_enemy (`self.Current Enemy`))
  (bind _ai_parry_damage (`self.AI Parry Damage`))
  (bind _parry_damage (`self.Parry Damage`))
  (bind _parry (`self.Parry`))
  (bind _current_enemy_2 (`self.Current Enemy`))
  (bind _ai__critic_damage (`self.AI +Critic Damage`))
  (bind __critic_damage (`self.+Critic Damage`))
  (bind _returnvalue (or (`self.Balanced Parry`) (`self.Offensive Parry`) (`self.Defensive Parry`)))
  (bind _selected (`/Game/Persona6/Blueprints/Characters/Player/BP_ThirdPersonCharacter.Selected` (`self.Player`)))
  (bind _result (`/Game/Persona6/Blueprints/Round_Widget.Result` (`self.Combat Widget`)))
  (bind _magic_active (`/Game/Persona6/Blueprints/Magics/Magic_Component.Magic Active` (`self.Magic Component`)))
  (bind _parrytype (`/Game/Persona6/Blueprints/Round_Widget.ParryType` (`self.Combat Widget`)))
  (bind _output (`|GetArrayItem` (`/Game/Persona6/Blueprints/Magics/Magic_Component.Magic Active` (`self.Magic Component`)) 3))
  (bind _output_2 (`|GetArrayItem` _magic_active 3))
  (if (or _counter_attack (`self.Parry Failed`))
    (`KismetSystemLibrary.PrintString` "PARRIED")
    (if _counter_attack
      (if (`|GetArrayItem` (`/Game/Persona6/Blueprints/Magics/Magic_Component.Magic Active` (`self.Magic Component`)) 3)
        (set `self.Parry Damage` (* _parry_damage 1.5))
        (else
          (set `self.Parry Damage` _parry_damage)))
      (`GameplayStatics.ApplyDamage` _current_enemy _parry_damage null _player_2)
      (elif _output
        (`GameplayStatics.ApplyDamage` _current_enemy _ai_parry_damage null _player_2)
        (else
          (`GameplayStatics.ApplyDamage` _player_2 _ai_parry_damage null _current_enemy))))
    (set `self.Balanced Parry` false)
    (set `self.Defensive Parry` false)
    (set `self.Counter Attack` false)
    (set `self.Parry Failed` false)
    (set `self.Counter Attack` false)
    (set `self.Parry Index` 0)
    (`TextBlock.SetText` _parrytype "")
    (else
      (`Widget.SetVisibility` _result "Visible")
      (if _selected
        (if (`self.Draw`)
          (`TextBlock.SetText` _result "=")
          (set `self.Draw` false)
          (if _parry
            (set `self.Balanced Parry` true)
            (`TextBlock.SetText` _parrytype "B \nA \nL \nA \nN \nC \nE \nD \n \nP \nA \nR \nR \nY")
            (set `self.Parry` false :!label _label)
            (`self.Next Round` :!label _label_2)
            (elif (`|GetArrayItem` _magic_active 9)
              (if _output_2 :!label _label_3
                (set `self.+Critic Damage` (* __critic_damage 1.5))
                (else
                  (set `self.+Critic Damage` __critic_damage)))
              (`GameplayStatics.ApplyDamage` _current_enemy_2 __critic_damage null _player)
              (else
                (`self.Next Round`))))
          (elif (not (`self.Player Won`))
            (`TextBlock.SetText` _result "<" :!label _label_4)
            (if (and _parry _selected)
              (set `self.Defensive Parry` true)
              (`TextBlock.SetText` _parrytype "D \nE \nF \nE \nN \nS \nI \nV \nE \n \nP \nA \nR \nR \nY")
              (goto _label)
              (elif _returnvalue
                (goto _label_2)
                (else
                  (if _output
                    (`GameplayStatics.ApplyDamage` _current_enemy_2 _ai__critic_damage null _player)
                    (elif _output_2
                      (goto _label_2)
                      (else
                        (`GameplayStatics.ApplyDamage` _player _ai__critic_damage null _current_enemy_2))))
                  (`TextBlock.SetText` _parrytype ""))))
            (else
              (`TextBlock.SetText` _result ">")
              (if _parry
                (set `self.Offensive Parry` true)
                (`TextBlock.SetText` _parrytype "O \nF \nF \nE \nN \nS \nI \nV \nE \n \nP \nA \nR \nR \nY")
                (goto _label)
                (elif _returnvalue
                  (goto _label_2)
                  (elif (`/Game/Persona6/Blueprints/Characters/BaseCharacter.Casted Magic` _player)
                    (`/Game/Persona6/Blueprints/Magics/Magic_Component.Casting Magic` (`self.Magic Component`) (`/Game/Persona6/Blueprints/Characters/BaseCharacter.Magic ID` _player))
                    (else
                      (goto _label_3))))))))
        (else
          (goto _label_4))))))

(fn `UserConstructionScript`)
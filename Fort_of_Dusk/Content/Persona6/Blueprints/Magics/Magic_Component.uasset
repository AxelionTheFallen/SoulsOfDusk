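; Magic component that casts a spell by ID in turn-based combat.
; CastingMagic resets matching inventory slots above index 24, then looks up the spell in the Magic_Data table.
; After a sound and delay, it records active state, turns and DoT by spell order, damages the current enemy and heals the player.
; It spawns the spell's VFX ahead of the combat camera and calls NextRound itself only for non-damaging spells.
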(event `Casting Magic`
  (params (`Magic ID` :type Name))
  (bind _asbp_third_person_character (cast `/Game/Persona6/Blueprints/Characters/Player/BP_ThirdPersonCharacter` (`GameplayStatics.GetPlayerCharacter` 0) :!pure true))
  (bind _aspersona_6_game_mode (cast `/Game/Persona6/Blueprints/Persona6_GameMode` (`GameplayStatics.GetGameMode`) :!pure true))
  (bind _asbp_third_person_character_2 (cast `/Game/Persona6/Blueprints/Characters/Player/BP_ThirdPersonCharacter` (`GameplayStatics.GetPlayerCharacter` 0) :!pure true))
  (bind _combatcamera (`/Game/Persona6/Blueprints/Characters/Player/BP_ThirdPersonCharacter.CombatCamera` _asbp_third_person_character))
  (bind _slot_structure (`/Game/Persona6/Blueprints/Inventory/InventorySystem.Slot Structure` (`Actor.GetComponentByClass` _asbp_third_person_character "/Game/Persona6/Blueprints/Inventory/InventorySystem.InventorySystem_C")))
  (for (_array_element _array_index) _slot_structure
    (if (and (== `Magic ID` (`.ItemId_7_2D41BED74C8CC8988AD074873717D6BC` (break `/Game/Persona6/Blueprints/Inventory/FSlotStruct` _array_element))) (> _array_index 24))
      (`KismetArrayLibrary.Array_Set` _slot_structure _array_index)))
  (bind _returnvalue (`|GetDataTableRow` "/Game/Persona6/Blueprints/Magics/Magic_Data.Magic_Data" `Magic ID`)
    (:`then`
      (`GameplayStatics.PlaySound2D` "/Game/ForFun/megumin-explosion_-sound-effect-made-with-Voicemod.megumin-explosion_-sound-effect-made-with-Voicemod" 1.0 1.0 0.0 null null)
      (`KismetSystemLibrary.Delay` 3.2)
      (bind (_turn _order _damage _dotdamage _heal _sfx _vfx) (break `/Game/Persona6/Blueprints/Magics/Magic_Structure` _returnvalue))
      (`KismetArrayLibrary.Array_Set` (`self.Magic Active`) _order true)
      (`KismetArrayLibrary.Array_Set` (`self.Magic Turn`) _order _turn)
      (`KismetArrayLibrary.Array_Set` (`self.Affliction Damage`) _order _dotdamage)
      (`GameplayStatics.ApplyDamage` (`/Game/Persona6/Blueprints/Persona6_GameMode.Current Enemy` _aspersona_6_game_mode) _damage)
      (`/Game/Persona6/Blueprints/Characters/BaseCharacter.Regen Heal` _asbp_third_person_character_2 _heal)
      (set `/Game/Persona6/Blueprints/Characters/BaseCharacter.Casted Magic` false _asbp_third_person_character_2)
      (`KismetSystemLibrary.PrintString` (`KismetSystemLibrary.GetDisplayName` _vfx))
      (`GameplayStatics.PlaySound2D` "/Game/ForFun/large-explosion-100420.large-explosion-100420" 1.0 1.0 0.0 null null)
      (`GameplayStatics.SpawnEmitterAtLocation` _vfx (+ (* (`SceneComponent.GetForwardVector` _combatcamera) 600.0) (`SceneComponent.K2_GetComponentLocation` _combatcamera) (* (`SceneComponent.GetUpVector` _combatcamera) 300.0)) (struct) (5.0 5.0 5.0))
      (if (<= _damage 0.0)
        (`/Game/Persona6/Blueprints/Persona6_GameMode.Next Round` _aspersona_6_game_mode)))))
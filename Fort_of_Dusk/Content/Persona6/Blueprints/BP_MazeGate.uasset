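; BP_MazeGate is a maze gate actor that slides a cube from its initial position to an End location.
; BeginPlay stores the cube's world location as Start.
; The Timer event passes through a DoOnce, so the move triggers only once, and plays a Timeline that lerps the cube's world location from Start to End without sweeping.
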(event `self.ReceiveBeginPlay`
  (set `self.Start` (`SceneComponent.K2_GetComponentLocation` (`self.Cube`))))

(event `Timer`
  (`/Engine/EditorBlueprintResources/StandardMacros.DoOnce` false
    (:`Completed`
      (bind (_direction _newtrack_0) (`Timeline|Timeline` :!via `PlayFromStart`)
        (:`Update`
          (`SceneComponent.K2_SetWorldLocation` (`self.Cube`) (`KismetMathLibrary.VLerp` (`self.Start`) (`self.End`) _newtrack_0) false false))))))

(fn `UserConstructionScript`)
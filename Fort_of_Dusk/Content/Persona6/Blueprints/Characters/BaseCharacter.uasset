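; Base character for round-based combat that handles incoming damage, heart-based health and death.
; On damage, one active MagicComponent effect negates the hit and another converts it to healing; otherwise Health drops.
; Surviving hits convert Health to heart and half-heart values for the empty SetHeart hook, then advance the GameMode's round.
; Lethal hits ragdoll the mesh with a radial impulse, then flag combat end and show the exit prompt.
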(event `self.ReceiveAnyDamage`
  (params (Damage :type "Float (single-precision)") (DamageType :type "DamageType Object Reference") (InstigatedBy :type "Controller Object Reference") (DamageCauser :type "Actor Object Reference"))
  (bind _health (`self.Health`))
  (bind _mesh (`self.Mesh`))
  (bind _aspersona_6_game_mode (cast `/Game/Persona6/Blueprints/Persona6_GameMode` (`GameplayStatics.GetGameMode`) :!pure true))
  (bind _returnvalue (- _health Damage))
  (bind _magic_active (`/Game/Persona6/Blueprints/Magics/Magic_Component.Magic Active` (`self.Magic_Component`)))
  (bind _starter (`/Game/Persona6/Blueprints/Round_Widget.Starter` (`/Game/Persona6/Blueprints/Persona6_GameMode.Combat Widget` _aspersona_6_game_mode)))
  (if (`|GetArrayItem` _magic_active)
    (`/Game/Persona6/Blueprints/Persona6_GameMode.Next Round` _aspersona_6_game_mode :!label _label)
    (else
      (`KismetSystemLibrary.PrintString` (`KismetStringLibrary.Conv_DoubleToString` Damage))
      (if (`|GetArrayItem` _magic_active 2)
        (set `self.Health` (+ Damage _health))
        (bind _returnvalue_2 (/ (- (stale _output_get) 10.0) 10.0))
        (bind _returnvalue_3 (`KismetMathLibrary.FFloor` _returnvalue_2))
        (bind _returnvalue_4 (+ (`KismetMathLibrary.Conv_IntToDouble` _returnvalue_3) 0.5))
        (`/Engine/EditorBlueprintResources/StandardMacros.CompareFloat` _returnvalue_2 _returnvalue_4 :!label _label_2
          (:`>`
            (set `self.Heart` (+ _returnvalue_3 1)))
          (:`==`
            (set `self.Heart` (+ _returnvalue_4 1.0) :!label _label_3)
            (set `self.Half` true))
          (:`<`
            (goto _label_3)))
        (`self.Set Heart`)
        (goto _label)
        (elif (<= _returnvalue 0.0)
          (set `self.Heart` -1.0)
          (`self.Set Heart`)
          (`PrimitiveComponent.SetCollisionEnabled` _mesh "QueryAndPhysics")
          (`PrimitiveComponent.SetSimulatePhysics` _mesh true)
          (`PrimitiveComponent.AddRadialForce` _mesh (+ (`self.K2_GetActorLocation`) (* (`self.GetActorForwardVector`) 75.0)) 500.0 100000.0 "RIF_Constant" true)
          (`KismetSystemLibrary.Delay` 1.0)
          (`TextBlock.SetText` _starter "Press space to end combat.")
          (`Widget.SetVisibility` _starter "Visible")
          (set `/Game/Persona6/Blueprints/Persona6_GameMode.Combat End` true _aspersona_6_game_mode)
          (else
            (bind _output_get (set `self.Health` _returnvalue))
            (goto _label_2)))))))

(event `Set Heart`)

(event `Regen Heal`
  (params (`Heal Amount` :type "Float (double-precision)")))

(fn `UserConstructionScript`)
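; Skeleton enemy NPC whose look, weapon and aura particle come from its MonsterID row in the MonstersData table on BeginPlay.
; The ChainedSkeleton variant also gets a neck chain and random limb chains.
; Rising skeletons hold a single-node animation while a recursive delay polls player distance.
; When the player is near, they switch to the AnimBP, play the rising montage with climbing sound, then tell Skeleton_AI to move.
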(event `self.ReceiveBeginPlay`
  (bind _mesh (`self.Mesh`))
  (bind _mesh_2 (`self.Mesh`))
  (bind _weapon (`self.Weapon`))
  (bind _returnvalue (`|GetDataTableRow` "/Game/Persona6/Blueprints/Characters/NPC/Agressive/MonstersData.MonstersData" (`self.Monster ID`))
    (:`then`
      (bind ((`WeaponMesh_116_A675AD994A01C7982E4477BCA5C7ED14` _weaponmesh) (`WeaponMaterial_117_F4A05A044F2969A5003CC6B0E37B669E` _weaponmaterial) (`Material1_140_73BA831E4B71AE242BD268B7698BAC29` _material1) (`OverlayMaterial_138_49AC26DB4BEB2C309326D3A52F7D38DD` _overlaymaterial) (`Particle_141_7FE93A764C7119EA9084CAADF2496744` _particle)) (break `/Game/Persona6/Blueprints/Characters/NPC/Agressive/MonstersStruct` _returnvalue))
      (`PrimitiveComponent.SetMaterial` _mesh 0 _material1)
      (`MeshComponent.SetOverlayMaterial` _mesh _overlaymaterial)
      (`StaticMeshComponent.SetStaticMesh` _weapon _weaponmesh)
      (`NiagaraComponent.SetAsset` (`self.AuraParticle`) _particle true)
      (`PrimitiveComponent.SetMaterial` _weapon 0 _weaponmaterial)
      (set `self.Pre Combat Location` (`self.K2_GetActorLocation`))
      (`|ExecutionSequence`
        (:`then_0`
          (if (== (`self.Monster ID`) "ChainedSkeleton")
            (`StaticMeshComponent.SetStaticMesh` (`self.ChainNeck`) "/Game/Persona6/Meshes/SM_ChainNeck.SM_ChainNeck")
            (for _ (range (+ (`KismetMathLibrary.RandomIntegerInRange` 1 3) 1))
              (switch `int` (`KismetMathLibrary.RandomIntegerInRange` 0 3)
                (:`0`
                  (`StaticMeshComponent.SetStaticMesh` (`self.ChainLeg_R`) "/Game/Persona6/Meshes/SM_ChainArm.SM_ChainArm"))
                (:`1`
                  (`StaticMeshComponent.SetStaticMesh` (`self.ChainArm_L`) "/Game/Persona6/Meshes/SM_ChainArm.SM_ChainArm"))
                (:`2`
                  (`StaticMeshComponent.SetStaticMesh` (`self.ChainArm_R`) "/Game/Persona6/Meshes/SM_ChainArm.SM_ChainArm"))
                (:`3`
                  (`StaticMeshComponent.SetStaticMesh` (`self.ChainLeg_L`) "/Game/Persona6/Meshes/SM_ChainArm.SM_ChainArm"))))))
        (:`then_1`
          (if (`self.Rising`)
            (`SkeletalMeshComponent.SetAnimationMode` _mesh_2 "AnimationSingleNode" true)
            (`SkeletalMeshComponent.SetAnimation` _mesh_2 "/Game/Persona6/Animations/AnimationSquences/SK_Skeleton_Sequence.SK_Skeleton_Sequence")
            (`self.Get Distance`)))
        (:`then_2`
          (`self.Set Data`)
          (set `self.Enemy 3D Combat Widget` (cast `/Game/Persona6/Blueprints/Characters/NPC/Agressive/EnemyAttackChooseWidget` (`WidgetComponent.GetWidget` (`self.3D Combat Widget`)) :!pure true)))))))

(event `Get Distance`
  (bind _climbingsound (`self.ClimbingSound`))
  (bind _mesh (`self.Mesh`))
  (`KismetSystemLibrary.Delay` 0.05)
  (if (`self.Rising`)
    (if (<= (`self.GetDistanceTo` (`GameplayStatics.GetPlayerCharacter` 0)) 1250.0)
      (`SkeletalMeshComponent.SetAnimationMode` _mesh "AnimationBlueprint" true)
      (`SkeletalMeshComponent.SetAnimInstanceClass` _mesh "/Game/Persona6/Blueprints/Characters/NPC/Agressive/Enemy_Skeleton_Anim.Enemy_Skeleton_Anim_C")
      (`AudioComponent.SetVolumeMultiplier` _climbingsound 1.0)
      (`AudioComponent.Play` _climbingsound 0.0)
      (bind _returnvalue (`self.PlayAnimMontage` "/Game/Persona6/Animations/AnimationSquences/Skeleton_Rising_Montage.Skeleton_Rising_Montage"))
      (set `self.Rising` false)
      (`KismetSystemLibrary.Delay` _returnvalue)
      (`/Game/Persona6/Blueprints/Characters/NPC/Agressive/Skeleton_AI.Move` (cast `/Game/Persona6/Blueprints/Characters/NPC/Agressive/Skeleton_AI` (`AIBlueprintHelperLibrary.GetAIController` self) :!pure true))
      (else
        (`self.Get Distance`)))))

(fn `UserConstructionScript`
  (`parent.UserConstructionScript`))
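; BP_MODULUS_SplinePlacer is a construction-script tool that repeats a chosen static mesh along a spline, in a MODULUS hedges and bushes folder.
; It derives segment length from the mesh's X bounds, allowing for centered pivots, and computes the count with an optional gap and full-length-only setting.
; Each segment is a deformed spline mesh with tangents clamped to mesh length and configurable collision, alongside an optional instruction text label.
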(fn `UserConstructionScript`
  (bind _textrender (`self.TextRender`))
  (bind _spline (`self.Spline`))
  (bind _returnvalue (`StaticMesh.GetBoundingBox` (`self.Spline Mesh`)))
  (bind _returnvalue_2 (`KismetMathLibrary.FTrunc` (/ (`SplineComponent.GetSplineLength` (`self.Spline`)) (+ (`self.Mesh X Length`) (`self.Offset`)))))
  ;[1 1 1] Get Mesh Size
  (set `self.Mesh X Length` (select `bool` (`self.Pivot in the Middle?`) :`false` (.x (`.Max` (break `Box` _returnvalue))) :`true` (* (.x (`.Max` (break `Box` _returnvalue))) 2.0)))
  (for _index (range (+ (select `bool` (`self.Only Full Length Mesh?`) :`false` _returnvalue_2 :`true` (- _returnvalue_2 1)) 1))
    ;[1 1 1] Add Mesh
    (bind _returnvalue_3 (`AddComponent|NODE_AddSplineMeshComponent-0`))
    (`StaticMeshComponent.SetStaticMesh` _returnvalue_3 (`self.Spline Mesh`))
    (`SplineMeshComponent.SetForwardAxis` _returnvalue_3 "X" true)
    (bind _returnvalue_4 (+ (* _index (`self.Mesh X Length`)) (* _index (`self.Offset`))))
    (bind _returnvalue_5 (+ (* (+ _index 1) (`self.Mesh X Length`)) (* _index (`self.Offset`))))
    (`SplineMeshComponent.SetStartAndEnd` _returnvalue_3 (`SplineComponent.GetLocationAtDistanceAlongSpline` _spline _returnvalue_4 "Local") (`KismetMathLibrary.ClampVectorSize` (`SplineComponent.GetTangentAtDistanceAlongSpline` _spline _returnvalue_4 "Local") 0.0 (`self.Mesh X Length`)) (`SplineComponent.GetLocationAtDistanceAlongSpline` _spline _returnvalue_5 "Local") (`KismetMathLibrary.ClampVectorSize` (`SplineComponent.GetTangentAtDistanceAlongSpline` _spline _returnvalue_5 "Local") 0.0 (`self.Mesh X Length`)) true)
    (`PrimitiveComponent.SetCollisionEnabled` _returnvalue_3 (`self.Collision Type`))
    (`SceneComponent.SetMobility` (`self.Spline`) (`self.Mobility?`))
    (`SceneComponent.K2_SetRelativeTransform` _textrender (`KismetMathLibrary.MakeTransform` (`SplineComponent.GetLocationAtSplinePoint` (`self.Spline`) _returnvalue_2 "Local") (struct :`Yaw` 180.0)) false false)
    (`SceneComponent.SetVisibility` _textrender (`self.Instruction?`) false)))